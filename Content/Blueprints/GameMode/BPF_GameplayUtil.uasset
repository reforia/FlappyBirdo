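; Blueprint function library of gameplay helpers for a Flappy Bird game, giving access to the game mode and its control state.
; GetFPGameMode returns the current game mode cast to GM_FlappyBird, or nothing when the cast fails.
; GetCanPlayerControlGame uses it to report whether the game is controllable, printing a critical on-screen error and returning false if that game mode is missing.
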(fn GetFPGameMode
  (bind _asgm_flappy_bird (Utilities|Casting|CastToGM_FlappyBird (Game|GetGameMode (LocalVariables|Get__WorldContext)))
    (:then
      (return _asgm_flappy_bird))
    (:CastFailed
      (return 0))))

(fn GetCanPlayerControlGame
  (bind ___worldcontext (LocalVariables|Get__WorldContext))
  (bind _gmref (CallFunction|GetFPGameMode ___worldcontext))
  (Utilities|IsValid _gmref
    (:Is%20Valid
      (return (Default|GetGameControllable _gmref)))
    (:Is%20Not%20Valid
      (Development|PrintString ___worldcontext "[Critical ERROR] Game Mode was not set to GM_FlappyBird" true true "(R=1.000000,G=0.000000,B=0.081419,A=1.000000)" 3e+01)
      (return false))))