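; Game mode for a Flappy Bird game that tracks the score and runs the session from start to level reload.
; BeginPlay broadcasts game start and enables the controllable flag, which is exposed through a getter.
; A player crash clears the flag, broadcasts session end and reloads FP_Main after a short delay, with debug prints standing in for end-game UI.
; Scoring events adjust the current score, clamped at zero.
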(event Custom|OnPlayerCrashed
  ;[1 1 1] Set Game Paused for now, the rest cleanup happens here before eng game Ui
  (Variables|Default|SetGameControllable false)
  (Development|PrintString "Game Over!")
  (CallFunction|OnGameplaySessionEnded)
  (Default|CallOnGameSessionEnd))

(event Custom|OnGameplaySessionEnded
  ;[1 1 1] Here, the player no longer can control the character, we are ready to show the end game UI
  (Development|PrintString "Game will restart in 3 secs")
  (Utilities|FlowControl|Delay 3.0)
  (Game|OpenLevel(byName) "FP_Main"))

(event Custom|OnPlayerScored
  (params (DeltaPoints :type Integer))
  (Variables|Default|SetCurrentScore (Math|Integer|Max(Integer) (+ (Variables|Default|GetCurrentScore) DeltaPoints))))

(event EventBeginPlay
  (Default|CallOnGameStart)
  (Variables|Default|SetGameControllable true))

(event EventTick
  (params (DeltaSeconds :type Float%20%28single-precision%29)))

(fn ConstructionScript)

(fn GetGameControllable
  (return (Variables|Default|GetGameControllable)))