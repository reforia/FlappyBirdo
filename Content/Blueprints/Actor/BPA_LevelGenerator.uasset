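; BPA_LevelGenerator is a level generator actor that produces an endless scrolling row of BPA_BlockingParts obstacles.
; On game start from the game mode it spawns an initial row, each block offset from the last by GapWidth.
; A looping timer, rather than Tick, shifts every part along local Y by a fixed step until session end.
; Parts overlapping PartsKillingZone are destroyed, and a replacement is appended after the last block.
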(event OnComponentBeginOverlap(PartsKillingZone)
  (params (OverlappedComponent :type Primitive%20Component%20Object%20Reference) (OtherActor :type Actor%20Object%20Reference) (OtherComp :type Primitive%20Component%20Object%20Reference) (OtherBodyIndex :type Integer) (bFromSweep :type Boolean) (SweepResult :type Hit%20Result%20Structure%20%28by%20ref%29))
  (if (Utilities|IsValid OtherActor)
    (bind _asbpa_blocking_parts (Utilities|Casting|CastToBPA_BlockingParts OtherActor))
    (CallFunction|RemoveandRefillBlock _asbpa_blocking_parts)))

(event Custom|InitializeLevel
  (for _index (range 1 (Variables|Default|GetInitialPillarCount))
    (CallFunction|GenerateNewBlock (Variables|Default|GetGapWidth)))
  (bind _returnvalue (Utilities|Time|SetTimerbyEvent (delegate Custom|UpdateParts) 0.016 true))
  (Variables|Default|SetUpdatePartTimerHandle _returnvalue))

(event Custom|UpdateParts
  (for _array_element (Variables|Default|GetPartsArray)
    (Transformation|AddActorLocalOffset _array_element (Math|Vector|MakeVector 0.0 (* (Variables|Default|GetPartsMovementSpeed) -1.0) 0.0) false false)))

(event Custom|StopLevel
  (Utilities|Time|ClearandInvalidateTimerbyHandle (Variables|Default|GetUpdatePartTimerHandle)))

(event EventBeginPlay
  (bind _gmref (CallFunction|GetFPGameMode))
  (Utilities|IsValid _gmref
    (:Is%20Valid
      (EventDispatchers|BindEventtoOnGameStart _gmref (delegate Custom|InitializeLevel))
      (EventDispatchers|BindEventtoOnGameSessionEnd _gmref (delegate Custom|StopLevel)))))

(event Collision|EventActorBeginOverlap
  (params (OtherActor :type Actor%20Object%20Reference)))

(event EventTick
  (params (DeltaSeconds :type Float%20%28single-precision%29)))

(fn ConstructionScript)

(fn GenerateNewBlock
  (params (SpawnGap :type Float%20%28double-precision%29))
  (bind _partsarray (Variables|Default|GetPartsArray))
  (bind _returnvalue (Utilities|Array|Length _partsarray))
  (if (> _returnvalue 0)
    (LocalVariables|SetNewBlockLocation (- (Transformation|GetActorLocation (Utilities|Array|Get(acopy) _partsarray (- _returnvalue 1))) (* (Math|Vector|GetRightVector (Variables|Default|GetLeftMostActorStartPoint)) SpawnGap)))
    (else
      (LocalVariables|SetNewBlockLocation (Transformation|GetWorldLocation (Variables|Default|GetLeftMostActorStartPoint)))))
  (bind _returnvalue_2 (Game|SpawnActorfromClass "/Game/Blueprints/Actor/BPA_BlockingParts.BPA_BlockingParts_C" (Math|Transform|MakeTransform (LocalVariables|GetNewBlockLocation) "0, 0, 0" "1.000000,1.000000,1.000000") "Undefined" 0 0))
  (Default|InitializeBlock _returnvalue_2 3e+02 -4e+02 4e+02 3.5e+02)
  (Utilities|Array|AddUnique (Variables|Default|GetPartsArray) _returnvalue_2)
  (Transformation|AttachComponentToComponent _returnvalue_2 (Variables|Default|GetBlockingPartsRoot) "None" "KeepWorld" "KeepWorld" "KeepWorld" true))

(fn RemoveandRefillBlock
  (params (PartToKill :type BPA%20Blocking%20Parts%20Object%20Reference))
  (if (Utilities|Array|ContainsItem (Variables|Default|GetPartsArray) PartToKill)
    (Utilities|Array|RemoveItem (Variables|Default|GetPartsArray) PartToKill)
    (else
      (Development|PrintString "[ERROR] A Blocking Part has been found but not in the managing array, attempting to destroy it" true true "(R=1.000000,G=0.000000,B=0.372514,A=1.000000)" 3e+01)))
  (Actor|DestroyActor PartToKill)
  (CallFunction|GenerateNewBlock (Variables|Default|GetGapWidth)))